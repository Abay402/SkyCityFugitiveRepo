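; Melee Blueprint that swaps a Paper2D flipbook between attack and idle animations.
; The Attack event sets the attack flipbook, then immediately compares the key frame index at its full play length, plus one, to one sixth of its frame count.
; A match switches straight to idle; the check never reads the current playback position or waits for the animation.
; BeginPlay, overlap, Tick and the construction script are empty.
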(event `Attack`
  (bind _rendercomponent (`self.RenderComponent`))
  (bind _attackanimation (`self.attackAnimation`))
  (`PaperFlipbookComponent.SetFlipbook` _rendercomponent _attackanimation)
  (bind _returnvalue (message `AnimationDataModel.GetPlayLength` _attackanimation))
  (bind _returnvalue_2 (message `AnimationDataModel.GetNumberOfFrames` _attackanimation))
  (if (== (+ (`PaperFlipbook.GetKeyFrameIndexAtTime` _attackanimation _returnvalue false) 1) (/ _returnvalue_2 6))
    (`PaperFlipbookComponent.SetFlipbook` _rendercomponent (`self.idleAnimation`))))

(fn `UserConstructionScript`)