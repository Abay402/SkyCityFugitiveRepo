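; BP_Enemy is an enemy actor that takes damage and stays dead once killed.
; HurtEnemy subtracts damage from Health and calls Dead at zero or below, which records the death in TestGameInstance's EnemyIsDead map and destroys the actor.
; On BeginPlay it destroys itself if that map marks it dead.
; Each enemy's map key is its first actor tag converted to an integer.
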(event `self.ReceiveBeginPlay`
  (bind _astest_game_instance (cast `/Game/Maps/TestGameInstance` (`GameplayStatics.GetGameInstance`)))
  (if (`BlueprintMapLibrary.Map_Find` (`/Game/Maps/TestGameInstance.enemyIsDead` _astest_game_instance) (`KismetStringLibrary.Conv_StringToInt` (`KismetStringLibrary.Conv_NameToString` (`|GetArrayItem` (`self.Tags`)))))
    (`self.K2_DestroyActor`)))

(event `Dead`
  (bind _astest_game_instance (cast `/Game/Maps/TestGameInstance` (`GameplayStatics.GetGameInstance`)))
  (`BlueprintMapLibrary.Map_Add` (`/Game/Maps/TestGameInstance.enemyIsDead` _astest_game_instance) (`KismetStringLibrary.Conv_StringToInt` (`KismetStringLibrary.Conv_NameToString` (`|GetArrayItem` (`self.Tags`)))) true)
  (`self.K2_DestroyActor`))

(event `HurtEnemy`
  (params (Damage :type Integer))
  (set `self.health` (- (`self.health`) Damage))
  (if (<= (`self.health`) 0)
    (`self.Dead`)))

(fn `UserConstructionScript`)