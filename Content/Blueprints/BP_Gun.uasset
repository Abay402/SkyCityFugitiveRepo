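; Mouse-aimed gun for a 2D side-view game, drawn with a flipbook and locked to a fixed Y plane.
; While active, Tick flips the controller yaw to the cursor's side and rotates the sprite along the deprojected mouse direction in XZ.
; ShootBullet spawns an effect and a bullet at the child actor, aiming the bullet at a point along the mouse ray flattened onto that plane.
; AttachArms swaps to the gun-with-arms flipbook.
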(event `self.ReceiveTick`
  (params (DeltaSeconds :type "Float (single-precision)"))
  (bind _rendercomponent (`self.RenderComponent`))
  (bind _returnvalue_x (`KismetMathLibrary.BreakVector` (`SceneComponent.K2_GetComponentLocation` (`self.RenderComponent`))))
  (bind (_worldlocation _worlddirection) (`PlayerController.DeprojectMousePositionToWorld` (`GameplayStatics.GetPlayerController` 0)))
  (bind (_returnvalue_x_2 _returnvalue_y _returnvalue_z) (`KismetMathLibrary.BreakVector` (`SceneComponent.K2_GetComponentLocation` _rendercomponent)))
  (if (`self.isActive`)
    (`/Engine/EditorBlueprintResources/StandardMacros.CompareFloat` (.x (`PlayerController.DeprojectMousePositionToWorld` (`GameplayStatics.GetPlayerController` 0))) _returnvalue_x
      (:`>`
        (`Controller.SetControlRotation` (`GameplayStatics.GetPlayerController` 0) (`KismetMathLibrary.MakeRotator` 0.0))
        (set `self.effectOffset` 0))
      (:`<`
        (`Controller.SetControlRotation` (`GameplayStatics.GetPlayerController` 0) (`KismetMathLibrary.MakeRotator` 0.0 0.0 180.0))
        (set `self.effectOffset` 0)))
    (`SceneComponent.K2_SetWorldLocation` _rendercomponent (`KismetMathLibrary.MakeVector` _returnvalue_x_2 51.0 _returnvalue_z) false false)
    (`SceneComponent.K2_SetWorldRotation` (`self.RenderComponent`) (`KismetMathLibrary.Conv_VectorToRotator` (`KismetMathLibrary.MakeVector` (.x _worlddirection) 0.0 (.z _worlddirection))) false false)))

(event `ShootBullet`
  (bind (_returnvalue_x _returnvalue_y _returnvalue_z) (`KismetMathLibrary.BreakVector` (`SceneComponent.K2_GetComponentLocation` (`self.ChildActor`))))
  (bind (_returnvalue_roll _returnvalue_pitch _returnvalue_yaw) (`KismetMathLibrary.BreakRotator` (`SceneComponent.K2_GetComponentRotation` (`self.RenderComponent`))))
  (bind (_worldlocation _worlddirection) (`PlayerController.DeprojectMousePositionToWorld` (`GameplayStatics.GetPlayerController` 0)))
  (bind (_returnvalue_x_2 _returnvalue_y_2 _returnvalue_z_2) (`KismetMathLibrary.BreakVector` (`SceneComponent.K2_GetComponentLocation` (`self.ChildActor`))))
  (bind (_returnvalue_x_3 _returnvalue_y_3 _returnvalue_z_3) (`KismetMathLibrary.BreakVector` (+ _worldlocation (* _worlddirection 200.0))))
  (`|SpawnActorFromClass` (`self.shootingEffect`) (`KismetMathLibrary.MakeTransform` (`KismetMathLibrary.MakeVector` (+ _returnvalue_x (`self.effectOffset`)) 53.0 _returnvalue_z) (`KismetMathLibrary.MakeRotator` _returnvalue_roll _returnvalue_pitch _returnvalue_yaw)) "Undefined" "MultiplyWithRoot" null null)
  (set `self.targetLocation` (`KismetMathLibrary.MakeVector` _returnvalue_x_3 51.0 _returnvalue_z_3))
  (set `self.spawnLocation` (`KismetMathLibrary.MakeVector` _returnvalue_x_2 51.0 _returnvalue_z_2))
  (set `self.bulletRotation` (`KismetMathLibrary.FindLookAtRotation` (`self.spawnLocation`) (`self.targetLocation`)))
  (`|SpawnActorFromClass` (`self.bulletType`) (`KismetMathLibrary.MakeTransform` (`KismetMathLibrary.MakeVector` _returnvalue_x_2 50.0 _returnvalue_z_2) (`self.bulletRotation`)) "Undefined" "MultiplyWithRoot" null null))

(event `AttachArms`
  (`PaperFlipbookComponent.SetFlipbook` (`self.RenderComponent`) "/Game/Assets/Flipbooks/Guns/GunWithArms1.GunWithArms1"))

(fn `UserConstructionScript`)